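; Player actor for a shooter, flying on a vertical plane oriented by its spawn yaw.
; A timeline spin-and-rise intro unlocks Tick movement, which eases input into swept horizontal and vertical motion with speed-based yaw.
; Held primary fire loops a timer spawning projectiles from two side points, while secondary fire spawns a laser gated by a timeline cooldown.
; Damage reduces health and reverses velocity as knockback, destroying the actor with a sound at zero.
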(event Custom|FireReset
  ;[1 1 1] Fire
  (CallFunction|PrimaryFire (Variables|Default|GetLeft))
  (CallFunction|PrimaryFire (Variables|Default|GetRight)))

(event Game|Damage|EventAnyDamage
  (params (Damage :type Float%20%28single-precision%29) (DamageType :type Damage%20Type%20Object%20Reference) (InstigatedBy :type Controller%20Object%20Reference) (DamageCauser :type Actor%20Object%20Reference))
  ;[1 1 1] Death
  (Variables|Default|SetHealth (Math|Float|Clamp(Float) (- (Variables|Default|GetHealth) Damage) 0.0 1e+02))
  (Variables|Default|SetHrztlSpeed (* (Variables|Default|GetHrztlSpeed) -2.0))
  (Variables|Default|SetVertSpeed (* (Variables|Default|GetVertSpeed) -2.0))
  (if (<= (Variables|Default|GetHealth) 0.0)
    (Audio|PlaySoundatLocation 0 (Transformation|GetActorLocation))
    (Actor|DestroyActor)))

(event EventBeginPlay
  ;[1 1 1] Platyer Spawn Animation
  (Variables|Default|SetYaw (.Yaw (Math|Rotator|BreakRotator (Transformation|GetActorRotation (Game|GetInstigator)))))
  (Variables|Default|SetSpawnLocation (Transformation|GetActorLocation))
  (bind _lerp (Timeline|SpawnAnimation Play)
    (:Update
      (Transformation|SetActorLocation (Math|Vector|Lerp(Vector) (Variables|Default|GetSpawnLocation) (+ (Variables|Default|GetSpawnLocation) "0, 0,60.000000") _lerp) false false)
      (Transformation|SetActorRotation (Math|Rotator|Lerp(Rotator) "0, 0, 0" (Math|Rotator|MakeRotator 0.0 0.0 (- 7.2e+02 (Variables|Default|GetYaw))) _lerp)))
    (:Finished
      (Variables|Default|SetbMovementEnabled true))))

(event EventTick
  (params (DeltaSeconds :type Float%20%28single-precision%29))
  ;[1 1 1] Player Movement
  (Variables|Default|SetDeltaSeconds DeltaSeconds)
  (if (Variables|Default|GetbMovementEnabled)
    (bind _returndirection (CallFunction|Movement (Variables|Default|GetHrztlSpeed) (Input|AxisValues|GetMoveRight)))
    (bind _returndirection_2 (CallFunction|Movement (Variables|Default|GetVertSpeed) (Input|AxisValues|GetMoveForward)))
    (Variables|Default|SetVertSpeed _returndirection_2)
    (Variables|Default|SetHrztlSpeed _returndirection)
    (Transformation|SetActorLocation (+ (Transformation|GetActorLocation) (Math|Vector|RotateVector (Math|Vector|MakeVector (Variables|Default|GetHrztlSpeed) 0.0 (Variables|Default|GetVertSpeed)) (Math|Rotator|MakeRotator 0.0 0.0 (Variables|Default|GetYaw)))) true false)
    (Transformation|SetActorRotation (Math|Interpolation|RInterpTo (Transformation|GetActorRotation) (Math|Rotator|MakeRotator 0.0 0.0 (+ (* (Variables|Default|GetHrztlSpeed) -1e+01) (Variables|Default|GetYaw))) (Variables|Default|GetDeltaSeconds) 0.0))))

(event Input|ActionEvents|InputActionPrimaryFire
  (params (Key :type Key%20Structure :default "AnyKey"))
  ;[1 1 1] Fire
  (:Pressed
    (bind _returnvalue (Utilities|Time|SetTimerbyFunctionName 0 "FireReset" 0.2 true))
    (Variables|Default|SetTimeHandle _returnvalue)
    (CallFunction|PrimaryFire (Variables|Default|GetLeft))
    (CallFunction|PrimaryFire (Variables|Default|GetRight)))
  (:Released
    (Utilities|Time|ClearandInvalidateTimerbyHandle (Variables|Default|GetTimeHandle))))

(event Input|ActionEvents|InputActionSecondaryFire
  (params (Key :type Key%20Structure :default "AnyKey"))
  ;[1 1 1] Fire Laser
  (:Pressed
    (if (Variables|Default|GetbLaserReady)
      (Variables|Default|SetbLaserReady false)
      (Game|SpawnActorfromClass "/Game/Blueprints/BPProjectileLaserUSSR.BPProjectileLaserUSSR_C" (Transformation|GetActorTransform) "Undefined" 0 "(R=0.000000,G=0.009551,B=0.945000,A=0.000000)" self)
      (Timeline|Timeline_0 Play
        (:Finished
          (Variables|Default|SetbLaserReady true))))))

(fn ConstructionScript)

(fn Movement
  (params (Speed :type Float%20%28single-precision%29) (Direction :type Float%20%28single-precision%29))
  (bind _output_get (Variables|Default|SetCurrentSpeed (Math|Interpolation|FInterpTo Speed (* (* Direction (Variables|Default|GetMovementSpeed)) 2.0) (Variables|Default|GetDeltaSeconds) 4.0)))
  (return _output_get))

(fn PrimaryFire
  (params (Location :type Scene%20Component%20Object%20Reference))
  (Game|SpawnActorfromClass "/Game/Blueprints/BPProjectile.BPProjectile_C" (Transformation|GetWorldTransform Location) "Undefined" 0 (Math|Color|MakeColor 0.6 0.3 0.6) (Math|Vector|MakeVector 0.0 0.0 7e+02) self))