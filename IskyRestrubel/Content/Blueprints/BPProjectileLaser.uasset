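; Laser projectile Blueprint that snaps to its owning actor and damages other actors it overlaps.
; The construction script creates a dynamic material, whose Color2 parameter BeginPlay sets to a fixed black, leaving ProjectileColor unused.
; A Movement timeline drives the mesh's scale and unswept relative location, then destroys the actor when finished.
; Overlaps ignore the owner and apply fixed damage without destroying the laser.
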(event OnComponentBeginOverlap(Projectile)
  (params (OverlappedComponent :type Primitive%20Component%20Object%20Reference) (OtherActor :type Actor%20Object%20Reference) (OtherComp :type Primitive%20Component%20Object%20Reference) (OtherBodyIndex :type Integer) (bFromSweep :type Boolean) (SweepResult :type Hit%20Result%20Structure%20%28by%20ref%29))
  ;[1 1 1] Collision Events
  (if (!= OtherActor (Variables|Default|GetProjectileOwner))
    (Game|Damage|ApplyDamage OtherActor 1.5e+02 0 0)
    (if (stale _bsuccess)
      _)))

(event EventBeginPlay
  (bind _projectile (Variables|Default|GetProjectile))
  ;[1 1 1] Set Material Color
  (Class|Actor|AttachRootComponenttoActor (Variables|Default|GetProjectileOwner) "None" "SnapToTarget" true)
  (Rendering|Material|SetVectorParameterValue :self (Variables|Default|GetProjectileMaterial) :ParameterName "Color2" :!class /Script/Engine.MaterialInstanceDynamic)
  (bind (_direction _extend _movement) (Timeline|Movement Play)
    (:Update
      (Transformation|SetWorldScale3D _projectile _extend)
      (Transformation|SetRelativeLocation _projectile _movement false false))
    (:Finished
      (Actor|DestroyActor))))

(fn ConstructionScript
  (bind _returnvalue (Rendering|Material|CreateDynamicMaterialInstance (Variables|Default|GetProjectile) 0 0 :!class /Script/Engine.PrimitiveComponent))
  (Variables|Default|SetProjectileMaterial _returnvalue))