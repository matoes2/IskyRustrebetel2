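; Game controller actor that runs the play loop: spawns and possesses the player ship, serves as the view target, and spawns enemies.
; A Tick-driven gate and Delay spawn random enemy classes at horizontal offsets, lengthening the interval up to a cap.
; Player death clears enemies and restarts through a second gate, which QuitGame closes first.
; A trigger destroys overlapping spawned enemies; enemy deaths play camera shake and sound.
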(event OnComponentBeginOverlap(Trigger)
  (params (OverlappedComponent :type Primitive%20Component%20Object%20Reference) (OtherActor :type Actor%20Object%20Reference) (OtherComp :type Primitive%20Component%20Object%20Reference) (OtherBodyIndex :type Integer) (bFromSweep :type Boolean) (SweepResult :type Hit%20Result%20Structure%20%28by%20ref%29))
  ;[1 1 1] Destroy off screen objects
  (if (Utilities|Array|ContainsItem (Variables|Default|GetSpawnedEnemies) OtherActor)
    (Actor|DestroyActor OtherActor)))

(event Custom|PlayCameraShake
  ;[1 1 1] Camera Shake
  (Camera|PlayWorldCameraShake 0 (Transformation|GetActorLocation) 0.0 5e+02))

(event Custom|ResetSpawnEnemies
  (bind _enemyspawnpoint (Variables|Default|GetEnemySpawnPoint))
  (bind _actorarray (Variables|Default|GetActorArray))
  (bind _maxhrztlspawnoffset (Variables|Default|GetMaxHrztlSpawnOffset))
  ;[1 1 1] Spawn Enemies at random locations
  (Utilities|FlowControl|Gate true) ; enters at Open
)

(event Custom|EnemyDestroyed
  (params (DestroyedActor :type Actor%20Object%20Reference))
  ;[1 1 1] Spawn Enemies at random locations
  (if (not (Variables|Default|GetbPlayerDead))
    (CallFunction|PlayCameraShake)
    (Utilities|FlowControl|DoOnce false :!label _label
      (:Completed
        (Audio|PlaySoundatLocation 0 "0, 0, 0")
        (goto _label Reset)))))

(event Custom|StopSpawningEnemies
  (bind _spawnedenemies (Variables|Default|GetSpawnedEnemies))
  (bind _enemyspawnpoint (Variables|Default|GetEnemySpawnPoint))
  (bind _actorarray (Variables|Default|GetActorArray))
  (bind _maxhrztlspawnoffset (Variables|Default|GetMaxHrztlSpawnOffset))
  ;[1 1 1] Spawn Enemies at random locations
  (for _array_element _spawnedenemies
    (Utilities|IsValid _array_element
      (:Is%20Valid
        (Actor|DestroyActor _array_element))))
  (Utilities|Array|Clear _spawnedenemies)
  (Utilities|FlowControl|Gate true) ; enters at Close
)

(event Custom|StartGame
  (bind _returnvalue (Game|GetPlayerController 0))
  (Variables|Default|SetbPlayerDead false)
  (Utilities|FlowControl|Sequence
    (:then_0
      (Variables|Default|SetSpawnInterval 1.0)
      (CallFunction|ResetSpawnEnemies)
      (bind _returnvalue_2 (Game|SpawnActorfromClass "/Game/Blueprints/BPPlayer.BPPlayer_C" (Transformation|GetWorldTransform (Variables|Default|GetPlayerSpawnPoint)) "Undefined" 0 0))
      (Variables|Default|SetPlayerShip _returnvalue_2)
      (Pawn|Possess _returnvalue (Variables|Default|GetPlayerShip))
      (Game|BindEventtoOnDestroyed (Variables|Default|GetPlayerShip) (delegate Custom|PlayerKilled))
      (Game|Player|SetViewTargetwithBlend _returnvalue self 0.0 "VTBlend_Linear" 0.0 true))
    (:then_1
      (Utilities|FlowControl|Gate true) ; enters at Open
    )))

(event Custom|PlayerKilled
  (params (DestroyedActor :type Actor%20Object%20Reference))
  (Variables|Default|SetbPlayerDead true)
  (CallFunction|StopSpawningEnemies)
  (Game|Player|SetViewTargetwithBlend (Game|GetPlayerController 0) self 0.0 "VTBlend_Linear" 0.0 false)
  (Utilities|FlowControl|Gate true
    (:Exit
      (CallFunction|StartGame))))

(event Custom|QuitGame
  (Utilities|FlowControl|Sequence
    (:then_0
      (Utilities|FlowControl|Gate true) ; enters at Close
    )
    (:then_1
      (Actor|DestroyActor (Variables|Default|GetPlayerShip))
      (CallFunction|PlayCameraShake))))

(event EventBeginPlay
  (CallFunction|StartGame))

(event EventTick
  (params (DeltaSeconds :type Float%20%28single-precision%29))
  (bind _enemyspawnpoint (Variables|Default|GetEnemySpawnPoint))
  (bind _actorarray (Variables|Default|GetActorArray))
  (bind _maxhrztlspawnoffset (Variables|Default|GetMaxHrztlSpawnOffset))
  ;[1 1 1] Spawn Enemies at random locations
  (Utilities|FlowControl|Gate true
    (:Exit
      (Utilities|FlowControl|Delay (Math|Random|RandomFloatinRange (Variables|Default|GetSpawnInterval) (+ (Variables|Default|GetSpawnInterval) 0.1)))
      (bind _returnvalue (Game|SpawnActorfromClass (Utilities|Array|Get(acopy) _actorarray (Math|Random|RandomInteger (Utilities|Array|Length _actorarray))) (Math|Transform|MakeTransform (+ (Transformation|GetWorldLocation _enemyspawnpoint) (Math|Vector|UnrotateVector (Math|Vector|MakeVector 0.0 (Math|Random|RandomFloatinRange (* _maxhrztlspawnoffset -1.0) _maxhrztlspawnoffset) 0.0) (Transformation|GetActorRotation))) (Transformation|GetWorldRotation _enemyspawnpoint) "1.000000,1,1") "Undefined" 0 0))
      (Utilities|Array|Add (Variables|Default|GetSpawnedEnemies) _returnvalue)
      (Game|BindEventtoOnDestroyed _returnvalue (delegate Custom|EnemyDestroyed))
      (Variables|Default|SetSpawnInterval (Math|Float|Clamp(Float) (+ (Variables|Default|GetSpawnInterval) 0.3) 0.7 1e+01)))))

(fn ConstructionScript
  (Transformation|SetRelativeLocation (Variables|Default|GetPlayerSpawnPoint) (Variables|Default|GetPlayerSpawnLocation) false false)
  (Transformation|SetRelativeLocation (Variables|Default|GetEnemySpawnPoint) (Variables|Default|GetEnemySpawnLocation) false false)
  (Transformation|SetRelativeLocation (Variables|Default|GetTrigger) (Variables|Default|GetTriggerLocation) false false))